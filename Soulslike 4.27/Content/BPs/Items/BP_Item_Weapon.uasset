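; Melee weapon item Blueprint that detects hits on enemies and deals damage for the current attack.
; SetAttackInfo stores the attack and clears the hit list.
; TraceHitbox sphere-traces between Start and End components on the Camera channel, skipping invulnerable enemies and the instigator, and records each hit to prevent repeats within an attack.
; DoDamage passes random min-max damage, scaled by the attack's modifier, to the target's TakeDamage, with debug prints throughout.
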(event EventBeginPlay
  (|CallParentFunction))

(event Collision|EventActorBeginOverlap
  (params (OtherActor :type Actor%20Object%20Reference))
  (|CallParentFunction OtherActor) ; This node is disabled and will not be called.\nDrag off pins to build functionality.
)

(event EventTick
  (params (DeltaSeconds :type Float%20%28single-precision%29))
  (|CallParentFunction DeltaSeconds) ; This node is disabled and will not be called.\nDrag off pins to build functionality.
)

(fn ConstructionScript
  (|CallParentFunction))

(fn GetDamage
  (return (Math|Random|RandomFloatinRange (Variables|Default|GetminDamage) (Variables|Default|GetmaxDamage))))

(fn SetAttackInfo
  (params (attackInfo :type S%20Char%20Attack%20Info%20Structure))
  (bind _output_get (Variables|Default|SetattackInfo attackInfo))
  (Utilities|Array|Clear (Variables|Default|GetHitActors))
  (Development|PrintString (Utilities|String|Append "INIT:  " (Utilities|String|EnumtoString (.attack _output_get))))
  (return))

(fn TraceHitbox
  (bind _outhit (Collision|SphereTraceByChannel (Transformation|GetWorldLocation (Variables|Default|GetStart)) (Transformation|GetWorldLocation (Variables|Default|GetEnd)) (Variables|Default|Getwidth) "TraceTypeQuery2" false (Variables|Default|GetHitActors) "None"))
  (for _index (range 0 (Utilities|Array|Length (Utilities|Array|MakeArray (.hitactor _outhit))))
    (bind _asbp_enemy_base (Utilities|Casting|CastToBP_Enemy_Base (Utilities|Array|Get(acopy) (Utilities|Array|MakeArray (.hitactor _outhit)) _index)))
    (if (and (not (Variables|/Game/BPs/Char/BP_Char_Base.BP_Char_Base_C|GetisInvulnerable _asbp_enemy_base)) (!= _asbp_enemy_base (Game|GetInstigator self)))
      (Utilities|Array|Add (Variables|Default|GetHitActors) _asbp_enemy_base)
      (CallFunction|DoDamage _asbp_enemy_base)
      (Development|PrintString (Utilities|String|Append (Utilities|String|ToString(Integer) _index) ". Hit: " (Utilities|GetDisplayName _asbp_enemy_base))))))

(fn DoDamage
  (params (target :type BP%20Char%20Base%20Object%20Reference))
  (bind _damage (CallFunction|GetDamage))
  (Development|PrintString (Utilities|GetDisplayName (Game|GetInstigator)) true true "(R=1.000000,G=0.000000,B=0.100000,A=1.000000)")
  (Default|TakeDamage target (Variables|Default|GetattackInfo) (* _damage (.damagemodifier (Variables|Default|GetattackInfo))) 1.0)
  (return))