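; Base character Blueprint for melee and ranged combat, holding HP, armor and poise stats, with stub hooks for HUD, blocking and targeting.
; TakeDamage triggers a game-pause hit stop, applies block, stun criticals and armor, then drains HP and poise toward death, stun or reaction montages chosen by Reactability.
; Timers delay and tick poise recovery.
; It also spawns projectiles and spells, and drives footstep and landing audio from floor physical-material traces.
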(event Custom|SetReactability
  (params (value :type Integer))
  (Variables|Default|SetReactability (Math|Integer|Clamp(Integer) value 0 4)))

(event Custom|EndBlock
  (Variables|Default|SetisBlocking false))

(event Custom|StartAttack
  (Variables|Default|SetisAttacking true))

(event Custom|InitPoiseRecovery
  ;[1 1 1] POISON MANAGMENT
  (bind _returnvalue (Utilities|Time|SetTimerbyEvent (delegate Custom|PoiseRecovery) 0.05 true)))

(event Custom|EndAttack
  (Variables|Default|SetisAttacking false)
  (Development|PrintString (Utilities|String|Append (Utilities|GetObjectName self) " END ATTACK")))

(event Custom|PoiseRecovery
  (bind _stats (Variables|Default|Getstats))
  ;[1 1 1] POISON MANAGMENT
  (bind _crntpoison (CallFunction|IncreasePoise (* (.poisonrecoverypersecond _stats) 0.05)))
  (if (>= _crntpoison (.maxpoise _stats))
    (CallFunction|StopPoiseRecovery)))

(event Custom|StopPoiseRecovery
  ;[1 1 1] POISON MANAGMENT
  (Utilities|Time|ClearandInvalidateTimerbyHandle (stale Custom|InitPoiseRecovery _returnvalue))
  (Utilities|Time|ClearandInvalidateTimerbyHandle (stale Custom|StopPoiseRecoveryDuringTime _returnvalue)))

(event Custom|StopPoiseRecoveryDuringTime
  ;[1 1 1] POISON MANAGMENT
  (Utilities|Time|ClearandInvalidateTimerbyHandle (stale Custom|InitPoiseRecovery _returnvalue))
  (bind _returnvalue (Utilities|Time|SetTimerbyEvent (delegate Custom|InitPoiseRecovery) (Variables|Default|GetpoiseFreezeTimer))))

(event Custom|StartBlock
  (Variables|Default|SetisBlocking true))

(event Custom|ActivateInvulnerability
  (Variables|Default|SetisInvulnerable true)
  (Development|PrintString (Utilities|String|Append (Utilities|GetObjectName self) " Is Invulnerable")))

(event Custom|DeactivateInvulnerability
  (Variables|Default|SetisInvulnerable false)
  (Development|PrintString (Utilities|String|Append (Utilities|GetObjectName self) " Is NOT Invulnerable")))

(event Custom|LandSound
  (bind _returnvalue (Transformation|GetActorLocation))
  (bind _jump_end (Variables|Default|GetJump_End))
  (bind _surface (Variables|Default|GetSurface))
  ;[1 1 1] JUMP END
  (Audio|Components|Audio|Play _jump_end 0.0)
  (Effects|Components|ParticleSystem|SetBoolParameter _jump_end "step_play" (Variables|Default|GetfootstepPlay))
  (Effects|Components|ParticleSystem|SetBoolParameter _jump_end "rattle_play" (Variables|Default|GetrattlePlay))
  (Effects|Components|ParticleSystem|SetBoolParameter _jump_end "voice_play" (Variables|Default|GetvoiceJumpPlay))
  ;[1 1 1] JUMPING VOLUME
  (Audio|Parameter|SetFloatParameter _jump_end "step_volume" (Variables|Default|GetfootstepVolume) :!class /Script/Engine.AudioComponent)
  (Audio|Parameter|SetFloatParameter _jump_end "rattle_volume" (Variables|Default|GetrattleVolume) :!class /Script/Engine.AudioComponent)
  (Audio|Parameter|SetFloatParameter _jump_end "voice_volume" (Variables|Default|GetvoiceJumpVolume) :!class /Script/Engine.AudioComponent)
  ;[1 1 1] Type of Floor
  (bind _outhit (Collision|LineTraceByChannel _returnvalue (- _returnvalue "0, 0,120.000000") "TraceTypeQuery1" false 0 "None"))
  (if (Utilities|Array|IsValidIndex _surface (Utilities|Array|FindItem _surface (.PhysMat (Collision|BreakHitResult _outhit))))
    (Effects|Components|ParticleSystem|SetIntParameter _jump_end "floor" (Utilities|Array|FindItem _surface (.PhysMat (Collision|BreakHitResult _outhit))))
    (Effects|Components|ParticleSystem|SetBoolParameter _jump_end "IsMale" false)
    (else
      (Effects|Components|ParticleSystem|SetIntParameter _jump_end "floor" 5))))

(event Custom|ResetPoise
  ;[1 1 1] POISON MANAGMENT
  (CallFunction|IncreasePoise (.maxpoise (Variables|Default|Getstats))))

(event Custom|HitPause
  (Development|PrintString "HIT PAUSE <-----------------" true true "(R=0.000000,G=0.452000,B=0.000000,A=1.000000)" 4.0)
  (Game|SetGamePaused true)
  (Utilities|FlowControl|Delay 0.0)
  (Utilities|FlowControl|Delay 0.0)
  (Utilities|FlowControl|Delay 0.0)
  (Utilities|FlowControl|Delay 0.0)
  (Utilities|FlowControl|Delay 0.0)
  (Utilities|FlowControl|Delay 0.0)
  (Game|SetGamePaused false))

(event Custom|DamageSound
  (bind _damage (Variables|Default|GetDamage))
  ;[1 1 1] Damage
  (Audio|Components|Audio|Play _damage 0.0)
  (Audio|Parameter|SetFloatParameter _damage "getHit_volume" (Variables|Default|GetgetHitVolume) :!class /Script/Engine.AudioComponent))

(event Custom|StepSound
  (params (maxVolume :type Boolean))
  (bind _returnvalue (Transformation|GetActorLocation))
  (bind _returnvalue_2 (Transformation|GetVelocity))
  (bind _footsteps (Variables|Default|GetFootsteps))
  (bind _surface (Variables|Default|GetSurface))
  (bind _returnvalue_3 (Math|Vector|VectorLength _returnvalue_2))
  ;[1 1 1] FOOTSTEPS
  (Audio|Components|Audio|Play _footsteps 0.0)
  (Effects|Components|ParticleSystem|SetBoolParameter _footsteps "step_play" (Variables|Default|GetfootstepPlay))
  (Effects|Components|ParticleSystem|SetBoolParameter _footsteps "rattle_play" (Variables|Default|GetrattlePlay))
  ;[1 1 1] Footsteps Volume
  (if (not maxVolume)
    (Audio|Parameter|SetFloatParameter _footsteps "step_volume" (* (Variables|Default|GetfootstepVolume) (Math|Float|MapRangeClamped _returnvalue_3 0.0 (Variables|Default|GetsprintSpeed) 0.0 0.7)) :!class /Script/Engine.AudioComponent)
    ;[1 1 1] Rattle Volume
    (Audio|Parameter|SetFloatParameter _footsteps "rattle_volume" (* (Variables|Default|GetrattleVolume) (Math|Float|MapRangeClamped _returnvalue_3 0.0 (Variables|Default|GetsprintSpeed) 0.1 0.7)) :!class /Script/Engine.AudioComponent)
    (else
      (Audio|Parameter|SetFloatParameter _footsteps "step_volume" (Variables|Default|GetfootstepVolume) :!class /Script/Engine.AudioComponent)
      (Audio|Parameter|SetFloatParameter _footsteps "rattle_volume" (Variables|Default|GetrattleVolume) :!class /Script/Engine.AudioComponent)))
  ;[1 1 1] Type of Floor
  (bind _outhit (Collision|LineTraceByChannel _returnvalue (- _returnvalue "0, 0,150.000000") "TraceTypeQuery1" false 0 "None"))
  (if (Utilities|Array|IsValidIndex _surface (Utilities|Array|FindItem _surface (.PhysMat (Collision|BreakHitResult _outhit))))
    (Effects|Components|ParticleSystem|SetIntParameter _footsteps "floor" (Utilities|Array|FindItem _surface (.PhysMat (Collision|BreakHitResult _outhit))))
    (else
      (Effects|Components|ParticleSystem|SetIntParameter _footsteps "floor" 5)))
  (Effects|Components|ParticleSystem|SetBoolParameter _footsteps "IsMale" false))

(event EventBeginPlay
  (bind _output_get (Variables|Default|Setstats (Utilities|Struct|MakeS_CharStats_ (.maxhp (Variables|Default|Getstats)) (.maxhp (Variables|Default|Getstats)) (.armorbase (Variables|Default|Getstats)) (.maxpoise (Variables|Default|Getstats)) (.maxpoise (Variables|Default|Getstats)) (.poisonrecoverypersecond (Variables|Default|Getstats)) (.maxstamina (Variables|Default|Getstats)) (.maxstamina (Variables|Default|Getstats)) (.hprecoverypersecond (Variables|Default|Getstats)) (.staminarecoverypersecond (Variables|Default|Getstats)) (.stabilitybase (Variables|Default|Getstats)))))
  (CallFunction|InitHUD _output_get)
  (if (Math|Float|NearlyEqual(Float) (Variables|Default|GetwalkSpeed) 0.0 0.1)
    (Variables|Default|SetwalkSpeed (* (Variables|Default|GetjogSpeed) 0.5))))

(fn ConstructionScript)

(fn Heal
  (params (healValue :type Float%20%28single-precision%29))
  (bind _output_get (Variables|Default|Setstats (Utilities|Struct|MakeS_CharStats_ (.maxhp (Variables|Default|Getstats)) (Math|Float|Clamp(Float) (+ healValue (.crnthp (Variables|Default|Getstats))) 0.0 (.maxhp (Variables|Default|Getstats))) (.armorbase (Variables|Default|Getstats)) (.maxpoise (Variables|Default|Getstats)) (.crntpoise (Variables|Default|Getstats)) (.poisonrecoverypersecond (Variables|Default|Getstats)) (.maxstamina (Variables|Default|Getstats)) (.crntstamina (Variables|Default|Getstats)) (.hprecoverypersecond (Variables|Default|Getstats)) (.staminarecoverypersecond (Variables|Default|Getstats)) (.stabilitybase (Variables|Default|Getstats)))))
  (CallFunction|IncreaseHPBar _output_get)
  (return))

(fn StartStun
  (if (not (Variables|Default|GetisDead))
    (Development|PrintString (Utilities|String|Append (Utilities|GetObjectName self) " is Stuned ---------------------------------<"))
    (Variables|Default|SetisStuned true)
    (CallFunction|StopCrntMontage)
    (CallFunction|EndAttack)
    (CallFunction|EndBlock)
    (CallFunction|EndDodge)
    (bind _returnvalue (Animation|PlayAnimMontage (Variables|Default|GethitAnim_Stuned) 1.0 "None"))
    (Utilities|Time|SetTimerbyFunctionName 0 "EndStun" _returnvalue)
    (return)))

(fn EndStun
  (Development|PrintString (Utilities|String|Append (Utilities|GetObjectName self) " is NO LONGER Stuned  ---------------------------------<"))
  (Variables|Default|SetisStuned false)
  (CallFunction|ResetPoise)
  (return))

(fn Die
  (Variables|Default|SetisDead true))

(fn BlockDamage
  (params (enterDamage :type Float%20%28single-precision%29))
  (return enterDamage))

(fn TakeDamage
  (params (attackInfo :type S%20Char%20Attack%20Info%20Structure) (damageReceived :type Float%20%28single-precision%29) (critical :type Float%20%28single-precision%29))
  (bind (_attack _staminacost _anim _damagemodifier _poisondamage _hitstrength) (Utilities|Struct|BreakS_CharAttackInfo_ attackInfo))
  (bind _hitanim_default (Variables|Default|GethitAnim_Default))
  (bind _hitanim_blocking (Variables|Default|GethitAnim_Blocking))
  (bind _hitanim_default_break (Variables|Default|GethitAnim_Default_Break))
  (bind _hitanim_blocking_break (Variables|Default|GethitAnim_Blocking_Break))
  (LocalVariables|SetlAttackInfo attackInfo)
  (LocalVariables|SetlInitDamage damageReceived)
  (LocalVariables|SetlCritical critical)
  (LocalVariables|SetlPoisonDamage _poisondamage)
  (LocalVariables|SetlHitStrength _hitstrength)
  (if (Math|Boolean|NORBoolean (Variables|Default|GetisDead) (Variables|Default|GetisInvulnerable))
    (CallFunction|HitPause)
    (CallFunction|DamageSound)
    (if (Variables|Default|GetisBlocking)
      (bind _finaldamage (CallFunction|BlockDamage (LocalVariables|GetlInitDamage)))
      (LocalVariables|SetlReceivedDamage _finaldamage)
      (else
        (LocalVariables|SetlReceivedDamage (LocalVariables|GetlInitDamage))
        (if (not (Variables|Default|GetisStuned))
          _
          (else
            (LocalVariables|SetlReceivedDamage (* (LocalVariables|GetlCritical) (LocalVariables|GetlReceivedDamage)))
            (Development|PrintString "Critical HIT" true true "(R=0.000000,G=0.452000,B=0.000000,A=1.000000)" 4.0)))))
    (bind _output_get (LocalVariables|SetlReceivedDamage (- (LocalVariables|GetlReceivedDamage) (* (LocalVariables|GetlReceivedDamage) (* (.armorbase (Variables|Default|Getstats)) 0.01)))))
    (if (<= _output_get 0.0)
      (LocalVariables|SetlReceivedDamage 0.0)
      (else
        (bind _die_ (CallFunction|DecreaseHP _output_get))))
    (Development|PrintString (Utilities|String|Append (Utilities|GetDisplayName self) " - has received \"" (Utilities|String|ToString(Float) (LocalVariables|GetlReceivedDamage)) "\" damage (" (Utilities|String|ToString(Float) (LocalVariables|GetlInitDamage)) "). Crnt HP: " (Utilities|String|ToString(Float) (.crnthp (Variables|Default|Getstats)))) true true "(R=0.000000,G=0.452000,B=0.000000,A=1.000000)" 4.0)
    (if (not _die_)
      (if (not (Variables|Default|GetisStuned))
        (bind _crntpoison (CallFunction|DecreasePoise (.poisondamage (LocalVariables|GetlAttackInfo))))
        (if (<= _crntpoison 0.0)
          (Development|PrintString "++++++++++++++++++")
          (CallFunction|StartStun)
          (elif (> (LocalVariables|GetlHitStrength) (Variables|Default|GetReactability))
            (CallFunction|StopCrntMontage)
            (CallFunction|EndAttack)
            (CallFunction|EndBlock)
            (CallFunction|EndDodge)
            (if (Variables|Default|GetisBlocking)
              (if (Utilities|IsValid _hitanim_blocking_break)
                (Animation|PlayAnimMontage _hitanim_blocking_break 1.0 (Variables|Default|GethitSectionName_Blocking_Break)))
              (Development|PrintString (Utilities|String|Append (Utilities|GetDisplayName self) "  " "HitAnim_Blocking_Break") true true "(R=0.000000,G=0.452000,B=0.000000,A=1.000000)" 5.0)
              (else
                (if (Utilities|IsValid _hitanim_default_break)
                  (Animation|PlayAnimMontage _hitanim_default_break 1.0 (Variables|Default|GethitSectionName_Default_Break)))
                (Development|PrintString (Utilities|String|Append (Utilities|GetDisplayName self) "  " "HitAnim_Default_Break") true true "(R=0.000000,G=0.452000,B=0.000000,A=1.000000)" 5.0)))
            (elif (Variables|Default|GetisBlocking)
              (if (Utilities|IsValid _hitanim_blocking)
                (Animation|PlayAnimMontage _hitanim_blocking 1.0 (Variables|Default|GethitSectionName_Blocking)))
              (Development|PrintString (Utilities|String|Append (Utilities|GetDisplayName self) "  " "HitAnim_Blocking") true true "(R=0.000000,G=0.452000,B=0.000000,A=1.000000)" 5.0)
              (else
                (CallFunction|EndBlock)
                (if (Math|Boolean|NORBoolean (Variables|Default|GetisAttacking) (Variables|Default|GetisDodging))
                  (CallFunction|EndAttack)
                  (CallFunction|EndDodge)
                  (if (Utilities|IsValid _hitanim_default)
                    (Animation|PlayAnimMontage _hitanim_default 1.0 (Variables|Default|GethitSectionName_Default)))
                  (Development|PrintString (Utilities|String|Append (Utilities|GetDisplayName self) "  " "HitAnim_Default") true true "(R=0.000000,G=0.452000,B=0.000000,A=1.000000)" 5.0))))))
        (else
          (Development|PrintString "hitAnim_Stuned" true true "(R=0.000000,G=0.452000,B=0.000000,A=1.000000)")))
      (else
        (CallFunction|Die)))))

(fn DecreaseHP
  (params (damageReceived :type Float%20%28single-precision%29))
  (if (not (Variables|Default|GetisInmortal))
    (bind _output_get (Variables|Default|Setstats (Utilities|Struct|MakeS_CharStats_ (.maxhp (Variables|Default|Getstats)) (Math|Float|Clamp(Float) (- (.crnthp (Variables|Default|Getstats)) damageReceived) 0.0 (.maxhp (Variables|Default|Getstats))) (.armorbase (Variables|Default|Getstats)) (.maxpoise (Variables|Default|Getstats)) (.crntpoise (Variables|Default|Getstats)) (.poisonrecoverypersecond (Variables|Default|Getstats)) (.maxstamina (Variables|Default|Getstats)) (.crntstamina (Variables|Default|Getstats)) (.hprecoverypersecond (Variables|Default|Getstats)) (.staminarecoverypersecond (Variables|Default|Getstats)) (.stabilitybase (Variables|Default|Getstats)))))
    (CallFunction|DecreaseHPBar _output_get damageReceived)
    (if (<= (.crnthp (Variables|Default|Getstats)) 0.0)
      (CallFunction|Die)
      (return true)
      (else
        (return false)))))

(fn IncreaseHPBar
  (params (stats :type S%20Char%20Stats%20Structure)))

(fn DecreaseHPBar
  (params (stats :type S%20Char%20Stats%20Structure) (damageReceied :type Float%20%28single-precision%29)))

(fn IncreasePoise
  (params (value :type Float%20%28single-precision%29))
  (Variables|Default|Setstats (Utilities|Struct|MakeS_CharStats_ (.maxhp (Variables|Default|Getstats)) (.crnthp (Variables|Default|Getstats)) (.armorbase (Variables|Default|Getstats)) (.maxpoise (Variables|Default|Getstats)) (Math|Float|Clamp(Float) (+ value (.crntpoise (Variables|Default|Getstats))) 0.0 (.maxpoise (Variables|Default|Getstats))) (.poisonrecoverypersecond (Variables|Default|Getstats)) (.maxstamina (Variables|Default|Getstats)) (.crntstamina (Variables|Default|Getstats)) (.hprecoverypersecond (Variables|Default|Getstats)) (.staminarecoverypersecond (Variables|Default|Getstats)) (.stabilitybase (Variables|Default|Getstats))))
  (return (Math|Float|Clamp(Float) (+ value (.crntpoise (Variables|Default|Getstats))) 0.0 (.maxpoise (Variables|Default|Getstats)))))

(fn DecreasePoise
  (params (value :type Float%20%28single-precision%29))
  (bind _output_get (Variables|Default|Setstats (Utilities|Struct|MakeS_CharStats_ (.maxhp (Variables|Default|Getstats)) (.crnthp (Variables|Default|Getstats)) (.armorbase (Variables|Default|Getstats)) (.maxpoise (Variables|Default|Getstats)) (Math|Float|Clamp(Float) (- (.crntpoise (Variables|Default|Getstats)) value) 0.0 (.maxpoise (Variables|Default|Getstats))) (.poisonrecoverypersecond (Variables|Default|Getstats)) (.maxstamina (Variables|Default|Getstats)) (.crntstamina (Variables|Default|Getstats)) (.hprecoverypersecond (Variables|Default|Getstats)) (.staminarecoverypersecond (Variables|Default|Getstats)) (.stabilitybase (Variables|Default|Getstats)))))
  (Development|PrintString (Utilities|String|Append (Utilities|GetDisplayName self) " - Poise: " (Utilities|String|ToString(Float) (.crntpoise _output_get))) true true "(R=0.755208,G=0.541201,B=0.000000,A=1.000000)")
  (CallFunction|StopPoiseRecoveryDuringTime)
  (return (.crntpoise _output_get)))

(fn InitHUD
  (params (Stats :type S%20Char%20Stats%20Structure)))

(fn StopCrntMontage
  (bind _mesh (Variables|Character|GetMesh))
  (bind _returnvalue (Components|SkeletalMesh|GetAnimInstance _mesh))
  (bind _returnvalue_2 (Animation|Montage|GetCurrentActiveMontage _returnvalue))
  (if (Utilities|IsValid _returnvalue_2)
    (Animation|StopAnimMontage _returnvalue_2)
    (return true)
    (else
      (return false))))

(fn ShootArrow
  (params (aInfo :type S%20Char%20Attack%20Info%20Structure))
  (bind _shootpos (CallFunction|GetShootPos))
  (Game|SpawnActorfromClass (Variables|Default|GetCrntProjectile) _shootpos "Undefined" 0 aInfo self))

(fn GetShootPos
  (return (Transformation|GetActorTransform)))

(fn SpawnSpell
  (params (Spell :type BP%20Spell%20Base%20Class%20Reference) (aInfo :type S%20Char%20Attack%20Info%20Structure))
  (bind _spellpos (CallFunction|GetSpellPos))
  (bind _returnvalue (Game|SpawnActorfromClass Spell _spellpos "Undefined" 0 aInfo self))
  (Development|PrintString (Utilities|GetClassDisplayName Spell)))

(fn GetSpellPos
  (return (Transformation|GetActorTransform)))

(fn EndDodge
  (Variables|Default|SetisDodging false))

(fn GetBlockingPercent
  (return 1.0))

(fn IsTargetable
  (return false))