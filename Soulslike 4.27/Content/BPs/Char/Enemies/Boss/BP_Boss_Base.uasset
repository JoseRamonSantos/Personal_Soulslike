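; Base boss enemy Blueprint whose awake and dead state persists through MyGameInstance.
; On BeginPlay it registers or restores that state, destroys itself if dead, or initializes its ActivationTrigger and mesh visibility.
; Activate wakes a sleeping boss, with an optional montage timing re-activation; once awake, it shows the UI_Boss health bar and starts the AI behavior tree.
; Damage only applies while active, and death clears the HUD, saves state and deactivates the trigger.
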(event EventBeginPlay
  (bind _activationtrigger (Variables|Default|GetactivationTrigger))
  (bind _activationtrigger_2 (Variables|Default|GetactivationTrigger))
  (|CallParentFunction)
  (if (Utilities|IsValidClass (.boss (Variables|Default|GetbossData)))
    _
    (else
      (Variables|Default|SetbossData (Utilities|Struct|MakeS_BossData (Utilities|GetClass self) false false))))
  (bind _asmy_game_instance (Utilities|Casting|CastToMyGameInstance (Game|GetGameInstance)))
  (bind _alreadyadded (Default|AddBossData _asmy_game_instance (Variables|Default|GetbossData)))
  (if _alreadyadded
    (bind _newdata (Default|GetSavedBossData _asmy_game_instance (Utilities|Struct|MakeS_BossData (Utilities|GetClass self) false false)))
    (Variables|Default|SetbossData _newdata))
  (if (.isdead (Variables|Default|GetbossData))
    (if (Utilities|IsValid _activationtrigger_2)
      (Default|Deactivate _activationtrigger_2))
    (Actor|DestroyActor)
    (else
      (Development|PrintString (Utilities|String|Append "+++++++++++++++++++++++++++++++++++++++++++++++++++     " (Utilities|String|ToString(Boolean) (.isawake (Variables|Default|GetbossData))) " / " (Utilities|String|ToString(Boolean) (.isdead (Variables|Default|GetbossData)))) true true "(R=0.000000,G=0.660000,B=1.000000,A=1.000000)" 4.0)
      (if (Utilities|IsValid _activationtrigger)
        (Default|Init _activationtrigger self (.isawake (Variables|Default|GetbossData)))
        (Rendering|SetVisibility (Variables|Character|GetMesh) (.isawake (Variables|Default|GetbossData)) false)))))

(event Collision|EventActorBeginOverlap
  (params (OtherActor :type Actor%20Object%20Reference))
  (|CallParentFunction OtherActor) ; This node is disabled and will not be called.\nDrag off pins to build functionality.
)

(fn ConstructionScript
  (|CallParentFunction))

(fn Activate
  (bind _self self)
  (bind _stats (Variables|Default|Getstats))
  (bind _returnvalue (AI|GetAIController _self))
  (if (.isawake (Variables|Default|GetbossData))
    (Variables|Default|SetisActive true)
    (bind _returnvalue_2 (UserInterface|CreateWidget "/Game/UI/UI_Boss.UI_Boss_C" (Game|GetPlayerController 0)))
    (bind _output_get (Variables|Default|SetgameHUD _returnvalue_2))
    (UserInterface|Viewport|AddtoViewport _output_get 0)
    (Default|Activate _output_get (Variables|Default|Getname) (.maxhp _stats) (.crnthp _stats))
    (bind _asaic_boss_base (Utilities|Casting|CastToAIC_Boss_Base _returnvalue))
    (Default|SetValuesandInitBT _asaic_boss_base)
    (Development|PrintString (Utilities|GetDisplayName _returnvalue))
    (else
      (CallFunction|Awake))))

(fn InitHUD
  (params (Stats :type S%20Char%20Stats%20Structure)))

(fn UpdateInstanceData
  (params (newData :type S%20Boss%20Data%20Structure))
  (Variables|Default|SetbossData (Utilities|Struct|MakeS_BossData (.boss (Variables|Default|GetbossData)) (.isawake newData) (.isdead newData)))
  (bind _asmy_game_instance (Utilities|Casting|CastToMyGameInstance (Game|GetGameInstance)))
  (Default|UpdateBossData _asmy_game_instance (Variables|Default|GetbossData)))

(fn Die
  (bind _bossdata (Variables|Default|GetbossData))
  (|CallParentFunction)
  (Widget|RemovefromParent (Variables|Default|GetgameHUD))
  (CallFunction|UpdateInstanceData (Utilities|Struct|MakeS_BossData (.boss _bossdata) (.isawake _bossdata) true))
  (if (Utilities|IsValid (Variables|Default|GetactivationTrigger))
    (Default|Deactivate (Variables|Default|GetactivationTrigger))))

(fn Awake
  (bind _bossdata (Variables|Default|GetbossData))
  (bind _awakeanim (Variables|Default|GetawakeAnim))
  (Development|PrintString (Utilities|String|Append (Utilities|GetDisplayName self) " - AWAKE ++++++++++++++++++++++++++++++") true true "(R=1.000000,G=0.301730,B=0.000000,A=1.000000)" 4.0)
  (Rendering|SetVisibility (Variables|Character|GetMesh) true false)
  (if (Utilities|IsValid _awakeanim)
    (bind _returnvalue (Animation|PlayAnimMontage _awakeanim 1.0 "None"))
    (Utilities|FlowControl|Sequence
      (:then_0
        (Utilities|Time|SetTimerbyFunctionName 0 "Activate" _returnvalue))
      (:then_1
        (if (not (.isawake (Variables|Default|GetbossData))) :!label _label
          (CallFunction|UpdateInstanceData (Utilities|Struct|MakeS_BossData (.boss _bossdata) true (.isdead _bossdata))))))
    (else
      (CallFunction|Activate)
      (goto _label))))

(fn DecreaseHPBar
  (params (stats :type S%20Char%20Stats%20Structure) (damageReceied :type Float%20%28single-precision%29))
  (|CallParentFunction stats damageReceied)
  (Default|Update (Variables|Default|GetgameHUD) (.crnthp (Variables|Default|Getstats)) damageReceied))

(fn TakeDamage
  (params (attackInfo :type S%20Char%20Attack%20Info%20Structure) (damageReceived :type Float%20%28single-precision%29) (critical :type Float%20%28single-precision%29))
  (if (Variables|Default|GetisActive)
    (|CallParentFunction attackInfo damageReceived critical)))