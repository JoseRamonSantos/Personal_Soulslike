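; Base projectile actor that damages characters on contact and plays an impact effect.
; On sphere overlap it ignores its instigator and other projectiles, then disables collision, stops movement, replaces its particles with a scaled impact emitter and clears its lifespan.
; BP_Char_Base targets take Damage scaled by AttackInfo's modifier, and the projectile attaches to their mesh before immediately being destroyed.
; Other hits leave the stopped actor in place.
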(event OnComponentBeginOverlap(Sphere)
  (params (OverlappedComponent :type Primitive%20Component%20Object%20Reference) (OtherActor :type Actor%20Object%20Reference) (OtherComp :type Primitive%20Component%20Object%20Reference) (OtherBodyIndex :type Integer) (bFromSweep :type Boolean) (SweepResult :type Hit%20Result%20Structure%20%28by%20ref%29))
  (bind _returnvalue (Transformation|GetActorTransform))
  (bind _projectilemovement (Variables|Default|GetProjectileMovement))
  (Development|PrintString (Utilities|String|Append " -->>>   " (Utilities|GetDisplayName OtherActor)))
  (if (!= OtherActor (Variables|Default|GetInstigator))
    (Utilities|Casting|CastToBP_Projectile_Base OtherActor
      (:CastFailed
        (Collision|SetCollisionEnabled (Variables|Default|GetSphere) "NoCollision")
        (Utilities|IsValid _projectilemovement
          (:Is%20Valid
            (Components|Activation|Deactivate _projectilemovement)
            (Components|DestroyComponent (Variables|Default|GetParticle%20System))
            (Effects|SpawnEmitteratLocation (Variables|Default|GetimpactParticle) (.location _returnvalue) (.rotation _returnvalue) (* "1.000000,1.000000,1.000000" (Variables|Default|GetimpactParticlesScale)))
            (Actor|SetLifeSpan self 0.0)
            (bind _asbp_char_base (Utilities|Casting|CastToBP_Char_Base OtherActor))
            (CallFunction|DoDamage _asbp_char_base)
            (Transformation|AttachComponentToComponent (Variables|/Script/Engine.Character|GetMesh _asbp_char_base) "None" "KeepWorld" "KeepWorld" "KeepWorld" false)
            (Actor|DestroyActor)))))))

(event EventBeginPlay)

(event EventTick
  (params (DeltaSeconds :type Float%20%28single-precision%29)))

(fn ConstructionScript)

(fn DoDamage
  (params (targetToDamage :type BP%20Char%20Base%20Object%20Reference))
  (Default|TakeDamage targetToDamage (Variables|Default|GetattackInfo) (* (Variables|Default|Getdamage) (.damagemodifier (Variables|Default|GetattackInfo))) 1.0))