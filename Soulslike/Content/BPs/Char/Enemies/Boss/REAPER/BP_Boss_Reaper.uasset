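; Reaper boss enemy character, built on a parent class that supplies its core behavior.
; It sets its move type on BeginPlay and exposes weapon hitbox endpoints and a spell transform from scene components.
; After the parent's damage handling, it has its boss AI controller check for phase two and three transitions against HP percentage thresholds.
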(event EventBeginPlay
  (|CallParentFunction)
  (CallFunction|ChangeMoveType "NewEnumerator1"))

(event Collision|EventActorBeginOverlap
  (params (OtherActor :type Actor%20Object%20Reference))
  (|CallParentFunction OtherActor) ; This node is disabled and will not be called.\nDrag off pins to build functionality.
)

(fn ConstructionScript
  (|CallParentFunction))

(fn GetStartandEndHitboxPos
  (return (Transformation|GetWorldLocation (Variables|Default|GetStart)) (Transformation|GetWorldLocation (Variables|Default|GetEnd))))

(fn GetSpellPos
  (return (Transformation|GetWorldTransform (Variables|Default|GetSpell))))

(fn TakeDamage
  (params (attackInfo :type S%20Char%20Attack%20Info%20Structure) (damageReceived :type Float%20%28single-precision%29) (critical :type Float%20%28single-precision%29))
  (bind _stats (Variables|Default|Getstats))
  (|CallParentFunction attackInfo damageReceived critical)
  (bind _asaic_boss_base (Utilities|Casting|CastToAIC_Boss_Base (AI|GetAIController (Components|GetOwner))))
  (Default|CheckPhase _asaic_boss_base (.crnthp _stats) (.maxhp _stats) 0.75 0.4))