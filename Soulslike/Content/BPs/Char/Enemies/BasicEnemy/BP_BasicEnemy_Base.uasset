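; Base Blueprint for basic enemies, managing an overhead HP bar widget and a Patrol, Chase and Attack state.
; ChangeState starts in Patrol, which hides the bar and uses controller desired rotation; Chase and Attack switch to controller yaw, with Attack also showing the bar.
; InitHUD caches the UI_EnemyHPBar widget for DecreaseHPBar updates.
; TakeDamage reveals the bar unless dead, and Die hides it.
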(event Custom|ShowHPBar
  (if (not (Variables|Default|GetisDead))
    (Rendering|SetVisibility (Variables|Default|GetHPBar) true false)))

(event Custom|HideHPBar
  (Rendering|SetVisibility (Variables|Default|GetHPBar) false false))

(event EventBeginPlay
  (|CallParentFunction)
  (CallFunction|HideHPBar)
  (CallFunction|ChangeState "NewEnumerator0"))

(event Collision|EventActorBeginOverlap
  (params (OtherActor :type Actor%20Object%20Reference))
  (|CallParentFunction OtherActor) ; This node is disabled and will not be called.\nDrag off pins to build functionality.
)

(event EventTick
  (params (DeltaSeconds :type Float%20%28single-precision%29))
  (|CallParentFunction DeltaSeconds) ; This node is disabled and will not be called.\nDrag off pins to build functionality.
)

(fn ConstructionScript
  (|CallParentFunction))

(fn InitHUD
  (params (Stats :type S%20Char%20Stats%20Structure))
  (bind _asui_enemy_hpbar (Utilities|Casting|CastToUI_EnemyHPBar (UserInterface|GetUserWidgetObject (Variables|Default|GetHPBar))))
  (bind _output_get (Variables|Default|SetwidgetHPBar _asui_enemy_hpbar))
  (Default|InitValues _output_get Stats))

(fn DecreaseHPBar
  (params (stats :type S%20Char%20Stats%20Structure) (damageReceied :type Float%20%28single-precision%29))
  (if (Utilities|IsValid (Variables|Default|GetwidgetHPBar))
    (Default|DecreaseHP (Variables|Default|GetwidgetHPBar) stats)
    (else
      (Development|PrintString "Unasigned EnemyHPBar. Enemy: DecreaseHPBar" true true "(R=1.000000,G=0.000000,B=0.000000,A=1.000000)" 5.0)))
  (return))

(fn ChangeState
  (params (newState :type e_basicEnemyStates%20Enum :default "NewEnumerator0"))
  (bind _charactermovement (Variables|Character|GetCharacterMovement))
  (bind _output_get (Variables|Default|SetcrntState newState))
  (switch Utilities|FlowControl|Switch|Switchone_basicEnemyStates _output_get
    (:NewEnumerator0
      (CallFunction|HideHPBar)
      (Variables|Default|SetbUseControllerRotationYaw false)
      (Variables|/Script/Engine.CharacterMovementComponent|SetbUseControllerDesiredRotation _charactermovement true))
    (:NewEnumerator1
      (Variables|Default|SetbUseControllerRotationYaw true :!label _label)
      (Variables|/Script/Engine.CharacterMovementComponent|SetbUseControllerDesiredRotation _charactermovement false))
    (:NewEnumerator2
      (CallFunction|ShowHPBar)
      (goto _label))))

(fn TakeDamage
  (params (attackInfo :type S%20Char%20Attack%20Info%20Structure) (damageReceived :type Float%20%28single-precision%29) (critical :type Float%20%28single-precision%29))
  (|CallParentFunction attackInfo damageReceived critical)
  (CallFunction|ShowHPBar))

(fn Die
  (|CallParentFunction)
  (CallFunction|HideHPBar))