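; Base enemy character Blueprint providing melee hit detection, movement speed tiers, targetability and death handling.
; TraceHitbox sphere-traces between placeholder endpoints, presumably overridden by children, and damages living, vulnerable BP_Char_Base targets using BaseDamage scaled by AttackInfo.
; HitActors is ignored by traces to prevent repeat hits until SetAttackInfo clears it for the next attack.
; Death disables capsule collision, stops the active montage and unpossesses the AI controller.
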(event EventBeginPlay
  (|CallParentFunction)
  (CallFunction|ChangeMoveType "NewEnumerator0"))

(event Collision|EventActorBeginOverlap
  (params (OtherActor :type Actor%20Object%20Reference))
  (|CallParentFunction OtherActor) ; This node is disabled and will not be called.\nDrag off pins to build functionality.
)

(event EventTick
  (params (DeltaSeconds :type Float%20%28single-precision%29))
  (|CallParentFunction DeltaSeconds) ; This node is disabled and will not be called.\nDrag off pins to build functionality.
)

(fn ConstructionScript
  (|CallParentFunction))

(fn GetDamage
  (return (Variables|Default|GetbaseDamage)))

(fn TraceHitbox
  (bind (_start _end) (CallFunction|GetStartandEndHitboxPos))
  (bind _outhit (Collision|SphereTraceByChannel _start _end (Variables|Default|GethitboxWidth) "TraceTypeQuery2" false (Variables|Default|GetHitActors) "ForOneFrame"))
  (for _index (range 0 (Utilities|Array|Length (Utilities|Array|MakeArray (.hitactor _outhit))))
    (bind _asbp_char_base (Utilities|Casting|CastToBP_Char_Base (Utilities|Array|Get(acopy) (Utilities|Array|MakeArray (.hitactor _outhit)) _index)))
    (if (Math|Boolean|ANDBoolean (not (Variables|/Game/BPs/Char/BP_Char_Base.BP_Char_Base_C|GetisDead _asbp_char_base)) (not (Variables|/Game/BPs/Char/BP_Char_Base.BP_Char_Base_C|GetisInvulnerable _asbp_char_base)) (!= _asbp_char_base self))
      (Utilities|Array|Add (Variables|Default|GetHitActors) _asbp_char_base)
      (CallFunction|DoDamage _asbp_char_base)
      (Development|PrintString (Utilities|String|Append (Utilities|String|ToString(Integer) _index) ". Hit: " (Utilities|GetDisplayName _asbp_char_base))))))

(fn DoDamage
  (params (target :type BP%20Char%20Base%20Object%20Reference))
  (bind _basedamage (CallFunction|GetDamage))
  (Development|PrintString (Utilities|String|ToString(Float) _basedamage) true true "(R=0.000000,G=0.364575,B=0.755208,A=1.000000)" 1e+01)
  (Default|TakeDamage target (Variables|Default|GetattackInfo) (* _basedamage (.damagemodifier (Variables|Default|GetattackInfo))) 1.0)
  (return))

(fn HastheActorBeenHit?
  (params (actors :type BP%20Char%20Base%20Object%20Reference))
  (bind _index (Utilities|FlowControl|ForLoopwithBreak 0 (Utilities|Array|Length (Variables|Default|GetHitActors)) :!label _label)
    (:LoopBody
      (if (== actors (Utilities|Array|Get(acopy) (Variables|Default|GetHitActors) _index))
        (LocalVariables|Setl_actorHit? true)
        (goto _label Break)
        (else
          (LocalVariables|Setl_actorHit? false))))
    (:Completed
      (return (LocalVariables|Getl_actorHit?)))))

(fn SetAttackInfo
  (params (attackInfo :type S%20Char%20Attack%20Info%20Structure))
  (Variables|Default|SetattackInfo attackInfo)
  (Development|PrintString "RESET")
  (Utilities|Array|Clear (Variables|Default|GetHitActors))
  (return))

(fn GetStartandEndHitboxPos
  (return "0.000000,0.000000,0.000000" "0.000000,0.000000,0.000000"))

(fn ChangeMoveType
  (params (NewParam :type E_MoveTypes%20Enum :default "NewEnumerator0"))
  (switch Utilities|FlowControl|Switch|SwitchonE_MoveTypes NewParam
    (:NewEnumerator0
      (Variables|/Script/Engine.CharacterMovementComponent|SetMaxWalkSpeed (Variables|Character|GetCharacterMovement) (Variables|Default|GetwalkSpeed)))
    (:NewEnumerator1
      (Variables|/Script/Engine.CharacterMovementComponent|SetMaxWalkSpeed (Variables|Character|GetCharacterMovement) (Variables|Default|GetjogSpeed)))
    (:NewEnumerator2
      (Variables|/Script/Engine.CharacterMovementComponent|SetMaxWalkSpeed (Variables|Character|GetCharacterMovement) (Variables|Default|GetsprintSpeed)))))

(fn Die
  (bind _self self)
  (bind _mesh (Variables|Character|GetMesh))
  (bind _returnvalue (AI|GetAIController _self))
  (bind _returnvalue_2 (Components|SkeletalMesh|GetAnimInstance _mesh))
  (bind _returnvalue_3 (Animation|Montage|GetCurrentActiveMontage _returnvalue_2))
  (|CallParentFunction)
  (Collision|SetCollisionEnabled (Variables|Default|GetCapsuleComponent) "NoCollision")
  (Utilities|IsValid _returnvalue_3
    (:Is%20Valid
      (Animation|Montage|MontageStop _returnvalue_2 0.0 _returnvalue_3))
    (:Is%20Not%20Valid
      _))
  (Utilities|IsValid _returnvalue
    (:Is%20Valid
      (AI|Navigation|StopMovement _returnvalue)
      (Pawn|UnPossess _returnvalue))))

(fn IsTargetable
  (return (not (Variables|Default|GetisDead))))