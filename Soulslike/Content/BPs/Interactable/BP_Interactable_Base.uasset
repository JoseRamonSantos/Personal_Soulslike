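; Base Blueprint for interactable objects that the player can use, with debug prints as placeholder behavior.
; Activate and Deactivate functions check an Activated flag, cast to BP_Player, then register or clear the object as the player's current interactable.
; Interact is gated by the same flag, while UseInteractable prints unconditionally; event graph and construction script are empty.
; GetName builds an identifier from display name and current level name.
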(event EventBeginPlay)

(event Collision|EventActorBeginOverlap
  (params (OtherActor :type Actor%20Object%20Reference)))

(event EventTick
  (params (DeltaSeconds :type Float%20%28single-precision%29)))

(fn ConstructionScript)

(fn UseInteractable
  (Development|PrintString (Utilities|String|Append "Player Interacted with:" (Utilities|GetDisplayName self))))

(fn ActivateInteractable
  (params (player :type Actor%20Object%20Reference))
  (if (Variables|Default|Getactivated)
    (bind _asbp_player (Utilities|Casting|CastToBP_Player player))
    (Default|EnableInteractable _asbp_player self)
    (Development|PrintString (Utilities|String|Append "Player can interact with: " (Utilities|GetDisplayName self)) true true "(R=0.000000,G=0.452000,B=0.000000,A=1.000000)" 4.0)))

(fn DeactivateIneractable
  (params (player :type Actor%20Object%20Reference))
  (if (Variables|Default|Getactivated)
    (bind _asbp_player (Utilities|Casting|CastToBP_Player player))
    (Default|DisenableInteractable _asbp_player)
    (Development|PrintString (Utilities|String|Append "Player can no longer interact with: " (Utilities|GetDisplayName self)) true true "(R=0.000000,G=0.452000,B=0.000000,A=1.000000)" 4.0)))

(fn Interact
  (if (Variables|Default|Getactivated)
    (Development|PrintString (Utilities|String|Append "Player interact with: " (Utilities|GetDisplayName self)))))

(fn GetName
  (bind _returnvalue (Game|GetCurrentLevelName true))
  (return (Utilities|String|Append (Utilities|GetDisplayName self) "_" _returnvalue)))