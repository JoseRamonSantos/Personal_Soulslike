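; Single-door interactable, openable from whichever sides are enabled, whose front and back boxes toggle interaction on overlap.
; Interact plays a timeline that rotates the mesh to OpenAngle on DoorAxis, lerping from its current rotation each update.
; It then clears Activated and saves it to MyGameInstance under the actor's name.
; BeginPlay registers the door there and, depending on the result, restores saved state, snapping opened doors open.
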(event OnComponentBeginOverlap(FrontBox)
  (params (OverlappedComponent :type Primitive%20Component%20Object%20Reference) (OtherActor :type Actor%20Object%20Reference) (OtherComp :type Primitive%20Component%20Object%20Reference) (OtherBodyIndex :type Integer) (bFromSweep :type Boolean) (SweepResult :type Hit%20Result%20Structure%20%28by%20ref%29))
  (if (Variables|Default|GetfrontOpenEnabled)
    (CallFunction|ActivateInteractable OtherActor)))

(event OnComponentEndOverlap(FrontBox)
  (params (OverlappedComponent :type Primitive%20Component%20Object%20Reference) (OtherActor :type Actor%20Object%20Reference) (OtherComp :type Primitive%20Component%20Object%20Reference) (OtherBodyIndex :type Integer))
  (if (Variables|Default|GetfrontOpenEnabled)
    (CallFunction|DeactivateIneractable OtherActor)))

(event OnComponentBeginOverlap(BackBox)
  (params (OverlappedComponent :type Primitive%20Component%20Object%20Reference) (OtherActor :type Actor%20Object%20Reference) (OtherComp :type Primitive%20Component%20Object%20Reference) (OtherBodyIndex :type Integer) (bFromSweep :type Boolean) (SweepResult :type Hit%20Result%20Structure%20%28by%20ref%29))
  (if (Variables|Default|GetbackOpenEnabled)
    (CallFunction|ActivateInteractable OtherActor)))

(event OnComponentEndOverlap(BackBox)
  (params (OverlappedComponent :type Primitive%20Component%20Object%20Reference) (OtherActor :type Actor%20Object%20Reference) (OtherComp :type Primitive%20Component%20Object%20Reference) (OtherBodyIndex :type Integer))
  (if (Variables|Default|GetbackOpenEnabled)
    (CallFunction|DeactivateIneractable OtherActor)))

(event Custom|OpenDoorInstant
  (bind _desiredrotation (CallFunction|GetRotations))
  (Transformation|SetRelativeRotation (Variables|Default|GetStaticMesh) _desiredrotation false false))

(event Custom|OpenDoor
  (Utilities|FlowControl|Delay 0.1)
  (bind _newtrack_0 (Timeline|OpenTL Play)
    (:Update
      (bind (_crntrotation _desiredrotation) (CallFunction|GetRotations))
      (Transformation|SetRelativeRotation (Variables|Default|GetStaticMesh) (Math|Rotator|Lerp(Rotator) _crntrotation _desiredrotation _newtrack_0 true) false false))))

(event Custom|UpdateData
  (bind _asmy_game_instance (Utilities|Casting|CastToMyGameInstance (Game|GetGameInstance)))
  (bind _name (CallFunction|GetName))
  (Default|UpdateDoorData _asmy_game_instance (Utilities|Struct|MakeS_DoorData _name (Variables|Default|Getactivated))))

(event EventBeginPlay
  (|CallParentFunction)
  (Components|Timeline|SetPlayRate (Variables|Default|GetOpenTL) (Variables|Default|GetopenRate))
  (bind _asmy_game_instance (Utilities|Casting|CastToMyGameInstance (Game|GetGameInstance)))
  (bind _name (CallFunction|GetName))
  (bind _exist_ (Default|AddDoorData _asmy_game_instance (Utilities|Struct|MakeS_DoorData _name (Variables|Default|Getactivated))))
  (if _exist_
    (bind _data (Default|GetSavedDoorData _asmy_game_instance (Utilities|Struct|MakeS_DoorData _name false)))
    (bind _output_get (Variables|Default|Setactivated (.activated _data)))
    (if (not _output_get)
      (CallFunction|OpenDoorInstant))))

(event Collision|EventActorBeginOverlap
  (params (OtherActor :type Actor%20Object%20Reference))
  (|CallParentFunction OtherActor) ; This node is disabled and will not be called.\nDrag off pins to build functionality.
)

(event EventTick
  (params (DeltaSeconds :type Float%20%28single-precision%29))
  (|CallParentFunction DeltaSeconds) ; This node is disabled and will not be called.\nDrag off pins to build functionality.
)

(fn ConstructionScript
  (|CallParentFunction))

(fn ActivateInteractable
  (params (player :type Actor%20Object%20Reference))
  (|CallParentFunction player))

(fn Interact
  (|CallParentFunction)
  (CallFunction|OpenDoor)
  (Variables|Default|Setactivated false)
  (CallFunction|UpdateData))

(fn GetRotations
  (bind _staticmesh (Variables|Default|GetStaticMesh))
  (bind _staticmesh_2 (Variables|Default|GetStaticMesh))
  (bind _staticmesh_3 (Variables|Default|GetStaticMesh))
  (bind _relativerotation (Variables|/Script/Engine.SceneComponent|GetRelativeRotation _staticmesh))
  (bind _relativerotation_2 (Variables|/Script/Engine.SceneComponent|GetRelativeRotation _staticmesh_3))
  (bind _relativerotation_3 (Variables|/Script/Engine.SceneComponent|GetRelativeRotation _staticmesh_2))
  (switch Utilities|FlowControl|Switch|SwitchonE_DoorAxis (Variables|Default|GetdoorAxis)
    (:NewEnumerator0
      (return (Variables|/Script/Engine.SceneComponent|GetRelativeRotation (Variables|Default|GetStaticMesh)) (Math|Rotator|MakeRotator (Variables|Default|GetopenAngle) (.pitch _relativerotation_3) (.yaw _relativerotation_3))))
    (:NewEnumerator1
      (return (Variables|/Script/Engine.SceneComponent|GetRelativeRotation (Variables|Default|GetStaticMesh)) (Math|Rotator|MakeRotator (.roll _relativerotation_2) (Variables|Default|GetopenAngle) (.yaw _relativerotation_2))))
    (:NewEnumerator2
      (return (Variables|/Script/Engine.SceneComponent|GetRelativeRotation (Variables|Default|GetStaticMesh)) (Math|Rotator|MakeRotator (.roll _relativerotation) (.pitch _relativerotation) (Variables|Default|GetopenAngle))))))