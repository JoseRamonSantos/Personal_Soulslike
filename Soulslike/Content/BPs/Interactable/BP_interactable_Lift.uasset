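; Interactable lift that moves a platform between StartPoint and EndPoint, either when LiftTrigger is overlapped or when called through Interact.
; Two timelines lerp the mesh, with play rates scaled by distance and Speed for consistent travel speed.
; Triggers at each end activate interaction for calling the lift; the first move enables both ends.
; Enabled flags and position are saved in MyGameInstance by actor name and restored on BeginPlay.
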(event OnComponentBeginOverlap(liftTrigger)
  (params (OverlappedComponent :type Primitive%20Component%20Object%20Reference) (OtherActor :type Actor%20Object%20Reference) (OtherComp :type Primitive%20Component%20Object%20Reference) (OtherBodyIndex :type Integer) (bFromSweep :type Boolean) (SweepResult :type Hit%20Result%20Structure%20%28by%20ref%29))
  (if (not (Variables|Default|GetisMoving))
    (bind (_start _end) (CallFunction|GetLiftPos))
    (if _start
      (CallFunction|SetMove true)
      (elif _end
        (CallFunction|SetMove false)))))

(event OnComponentBeginOverlap(StartTrigger)
  (params (OverlappedComponent :type Primitive%20Component%20Object%20Reference) (OtherActor :type Actor%20Object%20Reference) (OtherComp :type Primitive%20Component%20Object%20Reference) (OtherBodyIndex :type Integer) (bFromSweep :type Boolean) (SweepResult :type Hit%20Result%20Structure%20%28by%20ref%29))
  (CallFunction|ActivateInteractable OtherActor))

(event OnComponentEndOverlap(StartTrigger)
  (params (OverlappedComponent :type Primitive%20Component%20Object%20Reference) (OtherActor :type Actor%20Object%20Reference) (OtherComp :type Primitive%20Component%20Object%20Reference) (OtherBodyIndex :type Integer))
  (CallFunction|DeactivateIneractable OtherActor))

(event OnComponentBeginOverlap(EndTrigger)
  (params (OverlappedComponent :type Primitive%20Component%20Object%20Reference) (OtherActor :type Actor%20Object%20Reference) (OtherComp :type Primitive%20Component%20Object%20Reference) (OtherBodyIndex :type Integer) (bFromSweep :type Boolean) (SweepResult :type Hit%20Result%20Structure%20%28by%20ref%29))
  (CallFunction|ActivateInteractable OtherActor))

(event OnComponentEndOverlap(EndTrigger)
  (params (OverlappedComponent :type Primitive%20Component%20Object%20Reference) (OtherActor :type Actor%20Object%20Reference) (OtherComp :type Primitive%20Component%20Object%20Reference) (OtherBodyIndex :type Integer))
  (CallFunction|DeactivateIneractable OtherActor))

(event Custom|MoveToEnd
  (CallFunction|DisenableEndTrigger)
  (Variables|Default|SetisMoving true)
  (Utilities|FlowControl|Delay 0.1)
  (bind _newtrack_0 (Timeline|TLDoorToEnd PlayFromStart)
    (:Update
      (Transformation|SetWorldLocation (Variables|Default|GetStaticMesh) (Math|Vector|Lerp(Vector) (Transformation|GetWorldLocation (Variables|Default|GetStartPoint)) (Transformation|GetWorldLocation (Variables|Default|GetEndPoint)) _newtrack_0) false false))
    (:Finished
      (Variables|Default|SetisMoving false)
      (CallFunction|EnableStartTrigger))))

(event Custom|DisenableStartTrigger
  (bind _starttrigger (Variables|Default|GetStartTrigger))
  (bind _overlappingactors (Collision|GetOverlappingActors _starttrigger "/Game/BPs/Char/Player/BP_Player.BP_Player_C" :!class /Script/Engine.PrimitiveComponent))
  (Variables|/Script/Engine.PrimitiveComponent|SetbGenerateOverlapEvents _starttrigger false)
  (for _index (range 0 (Utilities|Array|Length _overlappingactors))
    (CallFunction|DeactivateIneractable (Utilities|Array|Get(acopy) _overlappingactors _index))))

(event Custom|MoveToStart
  (CallFunction|DisenableStartTrigger)
  (Variables|Default|SetisMoving true)
  (Utilities|FlowControl|Delay 0.1)
  (bind _newtrack_0 (Timeline|TLDoorToStart PlayFromStart)
    (:Update
      (Transformation|SetWorldLocation (Variables|Default|GetStaticMesh) (Math|Vector|Lerp(Vector) (Transformation|GetWorldLocation (Variables|Default|GetEndPoint)) (Transformation|GetWorldLocation (Variables|Default|GetStartPoint)) _newtrack_0) false false))
    (:Finished
      (Variables|Default|SetisMoving false)
      (CallFunction|EnableEndTrigger))))

(event Custom|MoveToStartInstant
  (Transformation|SetWorldLocation (Variables|Default|GetStaticMesh) (Transformation|GetWorldLocation (Variables|Default|GetStartPoint)) false false))

(event Custom|MoveToEndInstant
  (Transformation|SetWorldLocation (Variables|Default|GetStaticMesh) (Transformation|GetWorldLocation (Variables|Default|GetEndPoint)) false false))

(event Custom|UpdateData
  (bind _asmy_game_instance (Utilities|Casting|CastToMyGameInstance (Game|GetGameInstance)))
  (bind _name (CallFunction|GetName))
  (Default|UpdateLiftData _asmy_game_instance (Utilities|Struct|MakeS_LiftData _name (Variables|Default|GetstartEnabled) (Variables|Default|GetendEnabled) (Variables|Default|GetisAtStartPos))))

(event Custom|DisenableEndTrigger
  (bind _endtrigger (Variables|Default|GetEndTrigger))
  (bind _overlappingactors (Collision|GetOverlappingActors _endtrigger "/Game/BPs/Char/Player/BP_Player.BP_Player_C" :!class /Script/Engine.PrimitiveComponent))
  (Variables|/Script/Engine.PrimitiveComponent|SetbGenerateOverlapEvents _endtrigger false)
  (for _index (range 0 (Utilities|Array|Length _overlappingactors))
    (CallFunction|DeactivateIneractable (Utilities|Array|Get(acopy) _overlappingactors _index))))

(event Custom|EnableEndTrigger
  (bind _endtrigger (Variables|Default|GetEndTrigger))
  (bind _overlappingactors (Collision|GetOverlappingActors _endtrigger "/Game/BPs/Char/Player/BP_Player.BP_Player_C" :!class /Script/Engine.PrimitiveComponent))
  (Variables|/Script/Engine.PrimitiveComponent|SetbGenerateOverlapEvents _endtrigger true)
  (for _index (range 0 (Utilities|Array|Length _overlappingactors))
    (CallFunction|ActivateInteractable (Utilities|Array|Get(acopy) _overlappingactors _index))))

(event Custom|EnableStartTrigger
  (bind _starttrigger (Variables|Default|GetStartTrigger))
  (bind _overlappingactors (Collision|GetOverlappingActors _starttrigger "/Game/BPs/Char/Player/BP_Player.BP_Player_C" :!class /Script/Engine.PrimitiveComponent))
  (Variables|/Script/Engine.PrimitiveComponent|SetbGenerateOverlapEvents _starttrigger true)
  (for _index (range 0 (Utilities|Array|Length _overlappingactors))
    (CallFunction|ActivateInteractable (Utilities|Array|Get(acopy) _overlappingactors _index))))

(event EventBeginPlay
  (bind _endpoint (Variables|Default|GetEndPoint))
  (bind _startpoint (Variables|Default|GetStartPoint))
  (bind _speed (Variables|Default|Getspeed))
  (bind _returnvalue (Transformation|GetWorldLocation _endpoint))
  (bind _returnvalue_2 (Transformation|GetWorldLocation _startpoint))
  (bind _returnvalue_3 (- _returnvalue _returnvalue_2))
  (bind _returnvalue_4 (Math|Vector|VectorLength _returnvalue_3))
  (bind _returnvalue_5 (/ 1e+02 _returnvalue_4))
  (bind _returnvalue_6 (* _returnvalue_5 _speed))
  (|CallParentFunction)
  (Components|Timeline|SetPlayRate (Variables|Default|GetTLDoorToStart) _returnvalue_6)
  (Components|Timeline|SetPlayRate (Variables|Default|GetTLDoorToEnd) _returnvalue_6)
  (bind _start (CallFunction|GetLiftPos))
  (Variables|Default|SetisAtStartPos _start)
  (bind _asmy_game_instance (Utilities|Casting|CastToMyGameInstance (Game|GetGameInstance)))
  (bind _name (CallFunction|GetName))
  (bind _exist_ (Default|AddLiftData _asmy_game_instance (Utilities|Struct|MakeS_LiftData _name (Variables|Default|GetstartEnabled) (Variables|Default|GetendEnabled) (Variables|Default|GetisAtStartPos))))
  (if _exist_
    (bind _out_data (Default|GetSavedLiftData _asmy_game_instance (Utilities|Struct|MakeS_LiftData _name false false false)))
    (Variables|Default|SetstartEnabled (.startenabled _out_data))
    (Variables|Default|SetendEnabled (.endenabled _out_data))
    (bind _output_get (Variables|Default|SetisAtStartPos (.startpos _out_data)))
    (if _output_get
      (CallFunction|MovetoStartInstant)
      (else
        (CallFunction|MovetoEndInstant))))
  (if (Variables|Default|GetstartEnabled)
    (CallFunction|EnableStartTrigger)
    (else
      (CallFunction|DisenableStartTrigger)))
  (if (Variables|Default|GetendEnabled)
    (CallFunction|EnableEndTrigger)
    (else
      (CallFunction|DisenableEndTrigger)))
  (bind (_start_2 _end) (CallFunction|GetLiftPos))
  (if _start_2
    (CallFunction|DisenableStartTrigger)
    (elif _end
      (CallFunction|DisenableEndTrigger))))

(fn ConstructionScript
  (|CallParentFunction))

(fn Interact
  (|CallParentFunction)
  (if (not (Variables|Default|GetisMoving))
    (bind (_start _end) (CallFunction|GetLiftPos))
    (if _start
      (if (Variables|Default|GetendEnabled)
        (CallFunction|SetMove true))
      (elif _end
        (if (Variables|Default|GetstartEnabled)
          (CallFunction|SetMove false)
          (else
            (Development|PrintString "+++++++++++++++++++++++++++++++++++++")))
        (else
          (Development|PrintString "----------------------------------------------------"))))))

(fn GetLiftPos
  (if (Math|Vector|Equal(Vector) (Transformation|GetWorldLocation (Variables|Default|GetStaticMesh)) (Transformation|GetWorldLocation (Variables|Default|GetStartPoint)) 0.1)
    (return true false)
    (elif (Math|Vector|Equal(Vector) (Transformation|GetWorldLocation (Variables|Default|GetStaticMesh)) (Transformation|GetWorldLocation (Variables|Default|GetEndPoint)) 0.1)
      (return false true)
      (else
        (return false false)))))

(fn SetMove
  (params (toEnd :type Boolean))
  (if toEnd
    (CallFunction|MovetoEnd)
    (Variables|Default|SetisAtStartPos false)
    (else
      (CallFunction|MovetoStart)
      (Variables|Default|SetisAtStartPos true)))
  (Variables|Default|SetendEnabled true)
  (Variables|Default|SetstartEnabled true)
  (CallFunction|UpdateData))